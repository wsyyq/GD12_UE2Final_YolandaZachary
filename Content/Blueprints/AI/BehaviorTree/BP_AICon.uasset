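; AI controller that runs the BT_Goblin behavior tree on BeginPlay.
; Helper functions write the TargetLocation, SelfActor and TargetActor Blackboard keys and read the target back as an Actor.
; EmptyBlackBoard serves as death shutdown, resetting those three keys and stopping brain logic with reason "Dead".
; The event graph's calls to these helpers are unwired, so the controller itself never triggers them.
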(event EventBeginPlay
  (AI|RunBehaviorTree "/Game/Blueprints/AI/BehaviorTree/BT_Goblin.BT_Goblin"))

(event EventTick
  (params (DeltaSeconds :type Float%20%28single-precision%29)))

(fn ConstructionScript)

(fn UpdataTargetLocation
  (params (VectorValue :type Vector))
  (AI|Components|Blackboard|SetValueasVector (AI|GetBlackboard 0) (LocalVariables|GetTargetLocation) VectorValue))

(fn UpdataSelfActor
  (params (Actor :type Actor%20Object%20Reference))
  (AI|Components|Blackboard|SetValueasObject (AI|GetBlackboard 0) (LocalVariables|GetSelfActor) Actor))

(fn UpdataTargetActor
  (params (Actor :type Actor%20Object%20Reference))
  (AI|Components|Blackboard|SetValueasObject (AI|GetBlackboard 0) (LocalVariables|GetTargetActor) Actor))

(fn GetTargetActor
  (bind _asactor (Utilities|Casting|CastToActor (AI|Components|Blackboard|GetValueasObject (AI|GetBlackboard 0) (LocalVariables|GetTargetActorBB)))
    (:then
      (return _asactor))
    (:CastFailed
      (return 0))))

(fn EmptyBlackBoard
  (CallFunction|UpdataTargetLocation "0, 0, 0")
  (CallFunction|UpdataSelfActor)
  (CallFunction|UpdataTargetActor)
  (AI|Logic|StopLogic (Variables|Default|GetBrainComponent) "Dead"))