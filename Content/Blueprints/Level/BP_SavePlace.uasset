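; BP_SavePlace is an interactable level save point, judging by its name, that lights a fire when the player uses it.
; The PFire component is hidden on BeginPlay.
; The first E2Interact call reveals it, clears CanInteract and returns the PlayerAnimSpace world location as the player's teleport position with an interaction type.
; Later calls report it cannot be picked; no save logic appears in this Blueprint.
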(event EventBeginPlay
  (Development|SetHiddeninGame (Variables|Default|GetP_Fire) true false))

(fn ConstructionScript)

(fn E2Interact
  (if (Variables|Default|GetCanInteract)
    (Development|SetHiddeninGame (Variables|Default|GetP_Fire) false false)
    (Variables|Default|SetCanInteract false)
    (return true "NewEnumerator1" (Transformation|GetWorldLocation (Variables|Default|GetPlayerAnimSpace)) "0, 0, 0")
    (else
      (return false "NewEnumerator1" "0, 0, 0" "0, 0, 0"))))