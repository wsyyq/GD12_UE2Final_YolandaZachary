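; BP_Potions is a health potion that the player can pick up only when health is below maximum.
; An interaction box sets CanInteract while a BP_Character overlaps it and clears it on exit.
; E2Interact checks that flag, compares player 0's Health to MaxHealth, then returns CanPick and an interaction type to its caller.
; The healing itself is not applied in this Blueprint.
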(event OnComponentBeginOverlap(InteractBoxCollision)
  (params (OverlappedComponent :type Primitive%20Component%20Object%20Reference) (OtherActor :type Actor%20Object%20Reference) (OtherComp :type Primitive%20Component%20Object%20Reference) (OtherBodyIndex :type Integer) (bFromSweep :type Boolean) (SweepResult :type Hit%20Result%20Structure%20%28by%20ref%29))
  (Utilities|Casting|CastToBP_Character OtherActor)
  (Variables|Default|SetCanInteract true))

(event OnComponentEndOverlap(InteractBoxCollision)
  (params (OverlappedComponent :type Primitive%20Component%20Object%20Reference) (OtherActor :type Actor%20Object%20Reference) (OtherComp :type Primitive%20Component%20Object%20Reference) (OtherBodyIndex :type Integer))
  (Utilities|Casting|CastToBP_Character OtherActor)
  (Variables|Default|SetCanInteract false))

(fn ConstructionScript)

(fn E2Interact
  (bind _returnvalue (Game|GetPlayerCharacter 0))
  (bind _asbp_player_character (Utilities|Casting|CastToBP_PlayerCharacter _returnvalue))
  (if (Variables|Default|GetCanInteract)
    ;[0.15 0.15 0.15 0.5] 血量未满才能回血
    (if (< (Variables|/Game/Blueprints/BP_PlayerCharacter.BP_PlayerCharacter_C|GetHealth _asbp_player_character) (Variables|/Game/Blueprints/BP_PlayerCharacter.BP_PlayerCharacter_C|GetMaxHealth _asbp_player_character))
      (return true "NewEnumerator0")
      (else
        (return false "NewEnumerator0")))))