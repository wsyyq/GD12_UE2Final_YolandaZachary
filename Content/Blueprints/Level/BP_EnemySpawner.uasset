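; Level actor that spawns a goblin AI enemy when a BP_Character first overlaps its trigger box, with a small cap on total spawns.
; Each spawned enemy gets a Spawner reference back to this actor and is tracked in an alive-state map.
; OnDeath marks the given enemy dead and, once none remain alive, clears the map and spawns again until the cap is reached.
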(event OnComponentBeginOverlap(SpawnBox)
  (params (OverlappedComponent :type Primitive%20Component%20Object%20Reference) (OtherActor :type Actor%20Object%20Reference) (OtherComp :type Primitive%20Component%20Object%20Reference) (OtherBodyIndex :type Integer) (bFromSweep :type Boolean) (SweepResult :type Hit%20Result%20Structure%20%28by%20ref%29))
  (Utilities|Casting|CastToBP_Character OtherActor)
  (Utilities|FlowControl|DoOnce false
    (:Completed
      (CallFunction|OnSpawnGoblin))))

(event Custom|OnSpawnGoblin
  (bind _returnvalue (Transformation|GetActorTransform))
  ;[0.15 0.15 0.15 0.5] 哥布林生成器
  (Math|Integer|CompareInt (Variables|Default|GetSpawnTimes) 2
    (:<
      ;;[0.15 0.15 0.15 0.5] 在AI中，Owner为Controller
      (bind _returnvalue_2 (AI|SpawnAIFromClass (Variables|Default|GetGoblinClass) 0 (.location _returnvalue) (.rotation _returnvalue) false 0))
      ;[0.15 0.15 0.15 0.5] 通过Spawn来让之后能够在AI中调用对应的Spawn的函数
      (bind _asbp_enemy_character (Utilities|Casting|CastToBP_EnemyCharacter _returnvalue_2))
      (Variables|/Game/Blueprints/Enemy/BP_EnemyCharacter.BP_EnemyCharacter_C|SetSpawner _asbp_enemy_character self)
      ;[0.15 0.15 0.15 0.5] 加入到容器中
      (Utilities|Map|Add (Variables|Default|GetMapGoblinAlive) _returnvalue_2 true)
      (Math|Integer|IncrementInt (Variables|Default|GetSpawnTimes)))))

(event EventBeginPlay
  (Utilities|FlowControl|Delay 0.2))

(fn ConstructionScript)

(fn OnDeath
  (params (In%20Enemy :type Pawn%20Object%20Reference))
  (bind _mapgoblinalive (Variables|Default|GetMapGoblinAlive))
  ;[0.15 0.15 0.15 0.5] 将当前死掉的哥布林的Value设置为False
  (if (.Value (Utilities|Map|Find _mapgoblinalive In%20Enemy))
    (Utilities|Map|Add _mapgoblinalive In%20Enemy false)
    ;[0.15 0.15 0.15 0.5] 判断当前Map中变量是否都死了，有任一没死则值为True
    (bind _values (Utilities|Map|Values (Variables|Default|GetMapGoblinAlive)))
    (for _array_element _values
      (LocalVariables|SetIsAnyAlive (or _array_element (LocalVariables|GetIsAnyAlive))))
    (if (not (LocalVariables|GetIsAnyAlive))
      ;[0.15 0.15 0.15 0.5] 都死了则重新生成
      (Utilities|Map|Clear (Variables|Default|GetMapGoblinAlive))
      (CallFunction|OnSpawnGoblin)
      (return)
      (else
        (return)))))