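; Mission manager that runs five missions in a fixed order as a linear chain.
; After a short delay on BeginPlay it binds to the first mission's success and shows it; each success event binds, starts and shows the next one.
; It tracks the active mission in NowMission, exposes its name, description and type through GetNowMission, and calls CallMissionOver when the fifth succeeds.
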(event Custom|MissionOver1
  (bind _mission2 (Variables|Default|GetMission2))
  ;[0.15 0.15 0.15 0.5] 按顺序开启任务，共五个任务
  (EventDispatchers|BindEventtoMissionSuccess _mission2 (delegate Custom|MissionOver2))
  (Default|MissionStartandShowThis _mission2)
  (Variables|Default|SetNowMission _mission2))

(event Custom|MissionOver2
  (bind _mission3 (Variables|Default|GetMission3))
  ;[0.15 0.15 0.15 0.5] 按顺序开启任务，共五个任务
  (EventDispatchers|BindEventtoMissionSuccess _mission3 (delegate Custom|MissionOver3))
  (Default|MissionStartandShowThis _mission3)
  (Variables|Default|SetNowMission _mission3))

(event Custom|MissionOver3
  (bind _mission4 (Variables|Default|GetMission4))
  ;[0.15 0.15 0.15 0.5] 按顺序开启任务，共五个任务
  (EventDispatchers|BindEventtoMissionSuccess _mission4 (delegate Custom|MissionOver4))
  (Default|MissionStartandShowThis _mission4)
  (Variables|Default|SetNowMission _mission4))

(event Custom|MissionOver4
  (bind _mission5 (Variables|Default|GetMission5))
  ;[0.15 0.15 0.15 0.5] 按顺序开启任务，共五个任务
  (EventDispatchers|BindEventtoMissionSuccess _mission5 (delegate Custom|MissionOver5))
  (Default|MissionStartandShowThis _mission5)
  (Variables|Default|SetNowMission _mission5))

(event Custom|MissionOver5
  ;[0.15 0.15 0.15 0.5] 按顺序开启任务，共五个任务
  (Default|CallMissionOver))

(event EventBeginPlay
  (bind _mission1 (Variables|Default|GetMission1))
  ;[0.15 0.15 0.15 0.5] 按顺序开启任务，共五个任务
  (Utilities|FlowControl|Delay 0.2)
  (EventDispatchers|BindEventtoMissionSuccess _mission1 (delegate Custom|MissionOver1))
  (Default|MissionStartandShowThis _mission1)
  (Variables|Default|SetNowMission _mission1))

(fn ConstructionScript)

(fn GetNowMission
  (bind _nowmission (Variables|Default|GetNowMission))
  (return (Variables|/Game/Blueprints/Level/BP_Mission/BP_Mission.BP_Mission_C|GetMissionName _nowmission) (Variables|/Game/Blueprints/Level/BP_Mission/BP_Mission.BP_Mission_C|GetMissionDiscribe _nowmission) (Variables|/Game/Blueprints/Level/BP_Mission/BP_Mission.BP_Mission_C|GetMissionType _nowmission)))