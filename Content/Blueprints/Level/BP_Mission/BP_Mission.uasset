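; BP_Mission is a level-placed mission marker for either a kill-target or reach-destination objective.
; MissionStartAndShowThis reveals the initially hidden logo, enabling the overlap box only for destination missions; Tick yaws the logo using the player's camera boom position.
; The target's death event or the player character's overlap triggers completion, which hides the marker, disables collision, plays a stinger and calls MissionSuccess.
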(event OnComponentBeginOverlap(Box)
  (params (OverlappedComponent :type Primitive%20Component%20Object%20Reference) (OtherActor :type Actor%20Object%20Reference) (OtherComp :type Primitive%20Component%20Object%20Reference) (OtherBodyIndex :type Integer) (bFromSweep :type Boolean) (SweepResult :type Hit%20Result%20Structure%20%28by%20ref%29))
  ;[0.15 0.15 0.15 0.5] 到达目标任务完成
  (switch Utilities|FlowControl|Switch|SwitchonE_Mission (Variables|Default|GetMissionType)
    (:NewEnumerator0
      (Utilities|Casting|CastToBP_Character OtherActor)
      (Utilities|FlowControl|DoOnce false
        (:Completed
          (CallFunction|MissionSuccessandHideThis))))))

(event Custom|MissionSuccess_Kill
  ;[0.15 0.15 0.15 0.5] 击杀目标任务完成
  (CallFunction|MissionSuccessandHideThis))

(event EventBeginPlay
  ;[0.15 0.15 0.15 0.5] 开始游戏时任务隐藏
  (Rendering|SetVisibility (Variables|Default|GetMissionLOGO) false false)
  (Collision|SetCollisionEnabled (Variables|Default|GetBox) "NoCollision")
  (switch Utilities|FlowControl|Switch|SwitchonE_Mission (Variables|Default|GetMissionType)
    (:NewEnumerator1
      (bind _missiontarget (Variables|Default|GetMissionTarget)
        (:then
          (EventDispatchers|BindEventtoIDie _missiontarget (delegate Custom|MissionSuccess_Kill)))
        (:else)))))

(event EventTick
  (params (DeltaSeconds :type Float%20%28single-precision%29))
  ;[0.15 0.15 0.15 0.5] WBP面向玩家
  (if (Variables|Default|GetIsMissionStart)
    (Transformation|SetWorldRotation (Variables|Default|GetMissionLOGO) (Math|Rotator|MakeRotator 0.0 0.0 (.yaw (Math|Rotator|FindLookatRotation (Transformation|GetWorldLocation (Variables|/Script/MyARPG.MyARPGCharacter|GetCameraBoom (.AsBP%20Character (Utilities|Casting|CastToBP_Character (Game|GetPlayerCharacter 0))))) (Transformation|GetActorLocation)))) false false)))

(fn ConstructionScript)

(fn MissionSuccessandHideThis
  ;[0.15 0.15 0.15 0.5] 任务成功，标志消失
  (Rendering|SetVisibility (Variables|Default|GetMissionLOGO) false false)
  (Collision|SetCollisionEnabled (Variables|Default|GetBox) "NoCollision")
  (Audio|PlaySound2D "/Game/Assets/Sounds/Music/Stingers/A_Music_Stinger02.A_Music_Stinger02" 0.7 0.7 0.0 0 0)
  (Development|PrintString (Utilities|String|Append "任务" (Variables|Default|GetMissionName) "结束"))
  (Variables|Default|SetIsMissionStart false)
  (Variables|Default|SetIsMissionSuccess false)
  (Default|CallMissionSuccess))

(fn MissionStartandShowThis
  ;[0.15 0.15 0.15 0.5] 任务出现
  (Rendering|SetVisibility (Variables|Default|GetMissionLOGO) true false)
  (Development|PrintString (Utilities|String|Append "现在任务名：" (Variables|Default|GetMissionName)))
  (Variables|Default|SetIsMissionStart true)
  (switch Utilities|FlowControl|Switch|SwitchonE_Mission (Variables|Default|GetMissionType)
    (:NewEnumerator0
      (Collision|SetCollisionEnabled (Variables|Default|GetBox) "QueryOnly"))
    (:NewEnumerator1
      (Collision|SetCollisionEnabled (Variables|Default|GetBox) "NoCollision"))))