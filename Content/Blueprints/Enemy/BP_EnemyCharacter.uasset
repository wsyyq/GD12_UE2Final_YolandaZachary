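; Enemy character that wanders, makes melee attacks, reacts to hits and reports its death.
; Damage plays a hit montage, turns it toward the instigator and briefly blocks attacking; lethal damage calls IDie for the mission, sets a short lifespan and notifies its spawner.
; Melee plays one attack montage, guarded by flags that reset once no montage is playing.
; Patrol stores a random reachable nearby point as Destination, retrying recursively on failure.
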(event Game|Damage|EventAnyDamage
  (params (Damage :type Float%20%28single-precision%29) (DamageType :type Damage%20Type%20Object%20Reference) (InstigatedBy :type Controller%20Object%20Reference) (DamageCauser :type Actor%20Object%20Reference))
  (|CallParentFunction Damage DamageType InstigatedBy DamageCauser)
  (if (CallFunction|IsAlive)
    (Variables|Default|SetCanAttack false)
    (Animation|Montage|PlayMontage 0 "/Game/Animations/NPC/AM_Guardian_Hit.AM_Guardian_Hit" 0.8
      (:then
        ;[0.15 0.15 0.15 0.5] 看向打他的人
        (Transformation|SetActorRotation (Math|Rotator|MakeRotator 0.0 0.0 (.yaw (Math|Rotator|FindLookatRotation (Transformation|GetActorLocation) (Transformation|GetActorLocation InstigatedBy)))))
        (Utilities|FlowControl|Delay 0.05)
        (Variables|Default|SetCanAttack true))
      (:OnCompleted
        (Variables|Default|SetCanAttack true :!label _label))
      (:OnInterrupted
        (goto _label)))
    (else
      (CallFunction|OnDeath))))

(fn ConstructionScript
  (|CallParentFunction))

(fn DoMeleeAttack
  (params (MeleeAttackRate :type Float%20%28single-precision%29))
  (bind _mesh (Variables|Character|GetMesh))
  (bind _returnvalue (Components|SkeletalMesh|GetAnimInstance _mesh))
  (if (Variables|Default|GetIsMelee)
    ;[0.15 0.15 0.15 0.5] 如果此前无攻击的蒙太奇，则重置，并攻击一次
    (if (not (Class|AnimInstance|IsAnyMontagePlaying _returnvalue))
      (Variables|Default|SetMeleeIndex 0)
      (Variables|Default|SetIsMelee false)
      (CallFunction|DoMeleeAttack 1.0))
    (elif (not (> (Variables|Default|GetMeleeIndex) 0))
      ;[0.15 0.15 0.15 0.5] 普通攻击一次
      (Animation|Montage|MontagePlay _returnvalue "/Game/Animations/NPC/AM_Guardian_Attack.AM_Guardian_Attack" 1.0 "MontageLength" 0.0 true)
      (Variables|Default|SetMeleeIndex 1)
      (Variables|Default|SetIsMelee true))))

(fn SetDestination
  (params (Destination :type Vector))
  (Variables|Default|SetDestination Destination))

(fn GetNextNavPoint
  (bind _returnvalue (Transformation|GetActorLocation))
  (bind (_randomlocation _returnvalue_2) (AI|Navigation|GetRandomReachablePointinRadius _returnvalue 3e+02 0 0))
  ;[0.15 0.15 0.15 0.5] 巡逻，在附近乱逛
  (if _returnvalue_2
    (bind _output_get (LocalVariables|SetNewLocalVar _randomlocation))
    (CallFunction|SetDestination _output_get)
    (return _output_get)
    (else
      (CallFunction|GetNextNavPoint))))

(fn OnDeath
  ;[0.15 0.15 0.15 0.5] 告诉BP_Mission已完成
  (Default|CallIDie)
  ;[0.15 0.15 0.15 0.5] 类似Destroy
  (Actor|SetLifeSpan 2.0)
  (bind _asbp_enemy_spawner (Utilities|Casting|CastToBP_EnemySpawner (Variables|Default|GetSpawner)))
  (Default|OnDeath _asbp_enemy_spawner self))