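; Goblin enemy NPC that chases the first player's pawn and melee attacks it on reaching it.
; Tick, throttled by a short Delay, issues AI Move To while the goblin is alive and calls DoMeleeAttack on success.
; OnDamaged plays a Guardian hit-reaction montage.
; The randomized looping timer for EnemyAttack is disconnected, so attacks come only from the movement path.
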(event Custom|EnemyAttack
  (bind _animlength (CallFunction|DoMeleeAttack))
  (Utilities|FlowControl|Delay (- _animlength 0.1)))

(event EventBeginPlay
  (|CallParentFunction))

(event Collision|EventActorBeginOverlap
  (params (OtherActor :type Actor%20Object%20Reference))
  (|CallParentFunction OtherActor) ; This node is disabled and will not be called.\nDrag off pins to build functionality.
)

(event EventTick
  (params (DeltaSeconds :type Float%20%28single-precision%29))
  (|CallParentFunction DeltaSeconds)
  (Utilities|FlowControl|Delay 0.2)
  (if (CallFunction|IsAlive)
    (AI|AIMoveTo self "0, 0, 0" (Game|Player|GetPlayerPawn 0) 5.0 false
      (:OnSuccess
        (CallFunction|DoMeleeAttack)))))

(event EventOnDamaged
  (params (DamageAmount :type Float%20%28single-precision%29) (HitResult :type Hit%20Result%20Structure%20%28by%20ref%29) (InstigatorCharacter :type My%20ARPG%20Character%20Object%20Reference) (DamageCauser :type Actor%20Object%20Reference))
  (Animation|PlayAnimMontage "/Game/Animations/NPC/AM_Guardian_Hit.AM_Guardian_Hit" 1.0 "None"))

(fn ConstructionScript
  (|CallParentFunction))