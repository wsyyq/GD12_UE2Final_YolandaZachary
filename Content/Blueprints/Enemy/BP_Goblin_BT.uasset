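; BP_Goblin_BT is a behavior-tree goblin enemy that plays a hit montage when damaged.
; While alive, PawnSensing sends seen pawns and loud, nearby non-enemy noise locations to BP_AICon as targets.
; Delayed Tick polls for death, then shuts off sensing, empties the blackboard and notifies the player once for healing.
; The older timed melee attack and line-of-sight target logic are deprecated or disconnected.
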(event OnSeePawn(MyPawnSensing)
  (params (Pawn :type Pawn%20Object%20Reference))
  ;[0.15 0.15 0.15 0.5] 更新目标-看到
  (if (CallFunction|IsAlive)
    (bind _asbp_aicon (Utilities|Casting|CastToBP_AICon (AI|GetAIController self)))
    (Default|UpdataTargetActor _asbp_aicon Pawn)))

(event OnHearNoise(MyPawnSensing)
  (params (Instigator :type Pawn%20Object%20Reference) (Location :type Vector%20%28by%20ref%29 :default "0, 0, 0") (Volume :type Float%20%28single-precision%29))
  ;[0.15 0.15 0.15 0.5] 更新目标-听到
  (if (CallFunction|IsAlive)
    (if (not (Class|GameplayStatics|ObjectIsA "/Game/Blueprints/Enemy/BP_EnemyCharacter.BP_EnemyCharacter" (Utilities|GetClass Instigator)))
      (if (> Volume 4e+02)
        (if (<= (Math|Vector|VectorLength (- Location (Transformation|GetActorLocation))) 1.6e+03)
          ;;[0.15 0.15 0.15 0.5] 如果音量大于300，且该音量不是自己产生的，就把他记录下来
          (bind _asbp_aicon (Utilities|Casting|CastToBP_AICon (AI|GetAIController self)))
          (Default|UpdataTargetLocation _asbp_aicon Location))))))

(event Custom|EnemyAttack
  ;[0 0 0 0.5] 已废弃
  (bind _animlength (CallFunction|DoMeleeAttack 1.0))
  (Utilities|FlowControl|Delay (- _animlength 0.1)))

(event EventBeginPlay
  ;[0.15 0.15 0.15 0.5] 获得玩家BP
  (|CallParentFunction)
  (bind _asbp_character (Utilities|Casting|CastToBP_Character (Game|GetPlayerCharacter 0))
    (:then
      (Variables|Default|SetPlayer _asbp_character))
    (:CastFailed
      (Development|PrintString "BP_Goblin_BT：当前GameMode中玩家选择错误"))))

(event Collision|EventActorBeginOverlap
  (params (OtherActor :type Actor%20Object%20Reference))
  (|CallParentFunction OtherActor) ; This node is disabled and will not be called.\nDrag off pins to build functionality.
)

(event EventTick
  (params (DeltaSeconds :type Float%20%28single-precision%29))
  (bind _mypawnsensing (Variables|Default|GetMyPawnSensing))
  (|CallParentFunction DeltaSeconds)
  (Utilities|FlowControl|Delay 0.2)
  (if (not (CallFunction|IsAlive))
    ;[0.15 0.15 0.15 0.5] 死后清空行为树
    (Components|Activation|SetActive _mypawnsensing false false)
    (Components|Activation|Deactivate _mypawnsensing)
    (bind _asbp_aicon (Utilities|Casting|CastToBP_AICon (AI|GetAIController self)))
    (Default|EmptyBlackBoard _asbp_aicon)
    ;[0.15 0.15 0.15 0.5] 让玩家在AI死后回血
    (Utilities|FlowControl|DoOnce false
      (:Completed
        (Default|CallAIAlreadyDie (Variables|Default|GetPlayer))))))

(event EventOnDamaged
  (params (DamageAmount :type Float%20%28single-precision%29) (HitResult :type Hit%20Result%20Structure%20%28by%20ref%29) (InstigatorCharacter :type My%20ARPG%20Character%20Object%20Reference) (DamageCauser :type Actor%20Object%20Reference))
  ;[0.15 0.15 0.15 0.5] 受伤播放动画
  (Animation|PlayAnimMontage "/Game/Animations/NPC/AM_Guardian_Hit.AM_Guardian_Hit" 1.0 "None"))

(fn ConstructionScript
  (|CallParentFunction))