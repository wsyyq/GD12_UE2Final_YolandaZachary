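; Goblin enemy NPC that uses PawnSensing to chase and melee pawns it sees or investigate noises it hears.
; Sighting sets TargetPawn, while loud, nearby noises from non-enemy instigators set a Destination.
; A delayed Tick drives AIMoveTo toward either, attacks on reaching the target and forgets it when line of sight breaks.
; Damage plays a hit montage; the random-interval attack timer is unconnected.
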(event OnSeePawn(MyPawnSensing)
  (params (Pawn :type Pawn%20Object%20Reference))
  (Variables|Default|SetTargetPawn Pawn))

(event OnHearNoise(MyPawnSensing)
  (params (Instigator :type Pawn%20Object%20Reference) (Location :type Vector%20%28by%20ref%29 :default "0, 0, 0") (Volume :type Float%20%28single-precision%29))
  (if (not (Class|GameplayStatics|ObjectIsA "/Game/Blueprints/Enemy/BP_EnemyCharacter.BP_EnemyCharacter" (Utilities|GetClass Instigator)))
    (if (> Volume 5e+02)
      (if (<= (Math|Vector|VectorLength (- Location (Transformation|GetActorLocation))) 2e+03)
        ;[0.15 0.15 0.15 0.5] 如果音量大于300，且该音量不是自己产生的，就把他记录下来
        (CallFunction|SetDestination Location)))))

(event Custom|EnemyAttack
  (bind _animlength (CallFunction|DoMeleeAttack 1.0))
  (Utilities|FlowControl|Delay (- _animlength 0.1)))

(event EventBeginPlay
  (|CallParentFunction))

(event Collision|EventActorBeginOverlap
  (params (OtherActor :type Actor%20Object%20Reference))
  (|CallParentFunction OtherActor) ; This node is disabled and will not be called.\nDrag off pins to build functionality.
)

(event EventTick
  (params (DeltaSeconds :type Float%20%28single-precision%29))
  (|CallParentFunction DeltaSeconds)
  (Utilities|FlowControl|Delay 0.2)
  (if (CallFunction|IsAlive)
    (Utilities|FlowControl|Sequence
      (:then_0
        ;[0.15 0.15 0.15 0.5] 感知到目标再追逐
        (Utilities|IsValid (Variables|Default|GetTargetPawn)
          (:Is%20Valid
            (AI|AIMoveTo self "0, 0, 0" (Variables|Default|GetTargetPawn) 5.0 false
              (:OnSuccess
                (CallFunction|DoMeleeAttack 1.0))))
          (:Is%20Not%20Valid
            ;[0.15 0.15 0.15 0.5] 如果听到了destination，就前往destination位置
            (AI|AIMoveTo self (Variables|Default|GetDestination) 0 5.0 false))))
      (:then_1
        ;[0.15 0.15 0.15 0.5] 丢失目标：如果二者之间的连线为被阻挡，则会忘掉目标
        (Utilities|IsValid (Variables|Default|GetTargetPawn)
          (:Is%20Valid
            (bind _returnvalue (Class|MyPawnSensingComponent|HasLineOfSighttoBP (Variables|Default|GetMyPawnSensing) (Variables|Default|GetTargetPawn)))
            (if (not _returnvalue)
              (Variables|Default|SetTargetPawn 0))))))))

(event EventOnDamaged
  (params (DamageAmount :type Float%20%28single-precision%29) (HitResult :type Hit%20Result%20Structure%20%28by%20ref%29) (InstigatorCharacter :type My%20ARPG%20Character%20Object%20Reference) (DamageCauser :type Actor%20Object%20Reference))
  (Animation|PlayAnimMontage "/Game/Animations/NPC/AM_Guardian_Hit.AM_Guardian_Hit" 1.0 "None"))

(fn ConstructionScript
  (|CallParentFunction))