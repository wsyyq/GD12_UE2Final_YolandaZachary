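; Boss goblin enemy Blueprint that shrinks as it loses health, layered on logic inherited from its parent class.
; Each Tick sets uniform actor scale to twice the Health/MaxHealth ratio, comparing vector length against roughly √3 to clamp it at normal size from half health down.
; BeginPlay, overlap and construction only forward to the parent.
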(event EventBeginPlay
  (|CallParentFunction))

(event Collision|EventActorBeginOverlap
  (params (OtherActor :type Actor%20Object%20Reference))
  (|CallParentFunction OtherActor))

(event EventTick
  (params (DeltaSeconds :type Float%20%28single-precision%29))
  (bind _returnvalue (Math|Vector|MakeVector 2.0 2.0 2.0))
  (bind _health (Variables|Default|GetHealth))
  (bind _maxhealth (Variables|Default|GetMaxHealth))
  (bind _returnvalue_2 (/ _health _maxhealth))
  (bind _returnvalue_3 (* _returnvalue _returnvalue_2))
  (|CallParentFunction DeltaSeconds)
  (Math|Float|CompareFloat (Math|Vector|VectorLength _returnvalue_3) 1.732
    (:>
      (Transformation|SetActorScale3D self _returnvalue_3 :!label _label))
    (:==
      (goto _label))
    (:<
      (Transformation|SetActorScale3D self "1.000000,1.000000,1.000000"))))

(fn ConstructionScript
  (|CallParentFunction))