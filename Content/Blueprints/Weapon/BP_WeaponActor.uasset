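; Weapon actor that deals melee damage through a capsule hitbox and adds hit pause.
; Begin/EndWeaponAttack, noted as driven by NS_WeaponAttack, toggle capsule collision and attack state.
; Overlaps with actors of a different class than the instigator apply damage behind a DoOnce, reset after a delay on end overlap.
; A count-limited HitPause briefly slows global time after a short delay.
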(event OnComponentBeginOverlap(Capsule)
  (params (OverlappedComponent :type Primitive%20Component%20Object%20Reference) (OtherActor :type Actor%20Object%20Reference) (OtherComp :type Primitive%20Component%20Object%20Reference) (OtherBodyIndex :type Integer) (bFromSweep :type Boolean) (SweepResult :type Hit%20Result%20Structure%20%28by%20ref%29))
  (if (and (!= (Utilities|GetClass OtherActor) (Utilities|GetClass (Game|GetInstigator))) (Variables|WeaponDefaults|GetIsAttacking))
    (Utilities|FlowControl|DoOnce false
      (:Completed
        ;[0.15 0.15 0.15 0.5] Event Instigator为攻击者武器的控制器     DamageCauser为攻击者武器
        (Game|Damage|ApplyDamage OtherActor (Variables|Config|GetDamage) (Game|GetInstigatorController) self)
        ;[0.15 0.15 0.15 0.5] 播放时停效果
        (CallFunction|HitPause)
        (Development|PrintString "玩家攻击了哥布林")))))

(event OnComponentEndOverlap(Capsule)
  (params (OverlappedComponent :type Primitive%20Component%20Object%20Reference) (OtherActor :type Actor%20Object%20Reference) (OtherComp :type Primitive%20Component%20Object%20Reference) (OtherBodyIndex :type Integer))
  (Utilities|FlowControl|Delay (Variables|WeaponDefaults|GetEnableAttackDelayTime))
  (Utilities|FlowControl|DoOnce false) ; enters at Reset
)

(event Custom|BeginWeaponAttack
  (params (EnableAttackDelayCount :type Integer) (EnableAttackDelayTime :type Float%20%28double-precision%29))
  ;[0.15 0.15 0.15 0.5] 开始与结束攻击，判定位于NS_WeaponAttack
  (Variables|WeaponDefaults|SetEnableAttackDelayCount EnableAttackDelayCount)
  (Variables|WeaponDefaults|SetEnableAttackDelayTime EnableAttackDelayTime)
  (Variables|WeaponDefaults|SetIsAttacking true)
  (Collision|SetCollisionEnabled (Variables|Default|GetCapsule) "QueryOnly"))

(event Custom|EndWeaponAttack
  ;[0.15 0.15 0.15 0.5] 开始与结束攻击，判定位于NS_WeaponAttack
  (Variables|WeaponDefaults|SetIsAttacking false)
  (Collision|SetCollisionEnabled (Variables|Default|GetCapsule) "NoCollision"))

(event Custom|HitPause
  (if (and (> (Variables|WeaponDefaults|GetEnableAttackDelayCount) 0) (Variables|WeaponDefaults|GetEnableAttackDelay))
    (Math|Integer|DecrementInt (Variables|WeaponDefaults|GetEnableAttackDelayCount)
      (:%20%20
        (Utilities|FlowControl|Delay 0.1)
        ;[0.15 0.15 0.15 0.5] 将世界时间缩放至0.1倍
        (Utilities|Time|SetGlobalTimeDilation 0.1)
        ;[0.15 0.15 0.15 0.5] 在0.1倍下的0.01秒，即正常时间下的0.1秒
        (Utilities|FlowControl|Delay 0.01)
        (Utilities|Time|SetGlobalTimeDilation 1.0)))))

(event EventBeginPlay)

(event Collision|EventActorBeginOverlap
  (params (OtherActor :type Actor%20Object%20Reference)))

(event EventTick
  (params (DeltaSeconds :type Float%20%28single-precision%29)))

(fn ConstructionScript)