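; Player character for an action RPG with health, an equipped weapon and montage-based melee combos.
; On BeginPlay it spawns a weapon and attaches it to a mesh socket.
; AnyDamage clamps health and updates a camera-facing health bar, while OnDamaged plays a hit montage and material flash for BP_PlayerCharacter instigators.
; Melee combos pick a random next montage section from JumpSectionNotify during the combo window, parsing MeleeIndex from section names.
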(event EventBeginPlay
  ;[0.15 0.15 0.15 0.5] 开始时，在Sket欸之
  (CallFunction|CreateWeapon (Variables|Config|GetWeaponActorClass))
  (CallFunction|AttachWeapon 0 (Variables|Config|GetWeaponAttachSocket)))

(event Game|Damage|EventAnyDamage
  (params (Damage :type Float%20%28single-precision%29) (DamageType :type Damage%20Type%20Object%20Reference) (InstigatedBy :type Controller%20Object%20Reference) (DamageCauser :type Actor%20Object%20Reference))
  (bind _minhealth (Variables|HP|GetMinHealth))
  (bind _playerwidget (Variables|Default|GetPlayerWidget))
  (Class|MyARPGCharacter|HandleDamage Damage (Variables|Default|GetHit%20Result) 0 DamageCauser)
  ;[0.15 0.15 0.15 0.5] 受到伤害扣血
  (Math|Float|CompareFloat (- (Variables|HP|GetHealth) Damage) _minhealth
    (:>
      (Variables|HP|SetHealth (- (Variables|HP|GetHealth) Damage) :!label _label))
    (:==
      (goto _label))
    (:<
      (Variables|HP|SetHealth _minhealth)))
  ;[0.15 0.15 0.15 0.5] 更新血条值
  (Development|SetHiddeninGame _playerwidget (not (CallFunction|IsAlive)) false)
  (bind _aswbp_player_ui (Utilities|Casting|CastToWBP_PlayerUI (UserInterface|GetWidget _playerwidget)))
  (Default|SetHPPercentage _aswbp_player_ui (/ (Variables|HP|GetHealth) (Variables|HP|GetMaxHealth))))

(event EventTick
  (params (DeltaSeconds :type Float%20%28single-precision%29))
  (|CallParentFunction DeltaSeconds)
  ;[0.15 0.15 0.15 0.5] 更新血条UI朝向摄像机
  (Transformation|SetWorldRotation (Variables|Default|GetPlayerWidget) (Math|Rotator|MakeRotator 0.0 0.0 (.yaw (Math|Rotator|FindLookatRotation (Transformation|GetActorLocation) (Camera|GetCameraLocation (Variables|/Script/Engine.PlayerController|GetPlayerCameraManager (Game|GetPlayerController 0)))))) false false))

(event EventOnDamaged
  (params (DamageAmount :type Float%20%28single-precision%29) (HitResult :type Hit%20Result%20Structure%20%28by%20ref%29) (InstigatorCharacter :type My%20ARPG%20Character%20Object%20Reference) (DamageCauser :type Actor%20Object%20Reference))
  ;[0.15 0.15 0.15 0.5] 受到攻击动画
  (|CallParentFunction DamageAmount HitResult InstigatorCharacter DamageCauser)
  (Utilities|Casting|CastToBP_PlayerCharacter InstigatorCharacter)
  (Utilities|FlowControl|Sequence
    (:then_0
      (Animation|PlayAnimMontage "/Game/Characters/Animations/AM_React_Hit.AM_React_Hit" 1.0 "None"))
    (:then_1
      (CallFunction|PlayMaterialEffect "(R=1.000000,G=0.014359,B=0.000000,A=1.000000)" 1.0 (Variables|Character|GetMesh)))))

(fn ConstructionScript)

(fn IsAlive
  (return (> (Variables|HP|GetHealth) 0.0)))

(fn DoMeleeAttack
  (params (MeleeAttackRate :type Float%20%28single-precision%29))
  (if (Variables|Default|GetIsMelee)
    (CallFunction|JumpSectionforCombo)
    (if (not (Class|AnimInstance|IsAnyMontagePlaying (Components|SkeletalMesh|GetAnimInstance (Variables|Character|GetMesh))))
      ;[0.15 0.15 0.15 0.5] 播放蒙太奇的某一片段
      (bind _returnvalue (Animation|PlayAnimMontage "/Game/Characters/Animations/AM_Attack_Axe.AM_Attack_Axe" MeleeAttackRate "Combo1" :!label _label))
      (Variables|Default|SetIsMelee true)
      (Variables|Default|SetMeleeIndex 1)
      (return _returnvalue))
    (elif (not (> (Variables|Default|GetMeleeIndex) 0))
      (goto _label))))

(fn JumpSectionforCombo
  (bind _jumpsectionnotify (Variables|Default|GetJumpSectionNotify))
  (bind _mesh (Variables|Character|GetMesh))
  (bind _returnvalue (Components|SkeletalMesh|GetAnimInstance _mesh))
  (bind _jumpsections (Variables|/Game/Blueprints/AnimNotifies/NS_JumpSection.NS_JumpSection_C|GetJumpSections _jumpsectionnotify))
  (bind _returnvalue_2 (Utilities|Array|Length _jumpsections))
  (bind _returnvalue_3 (Animation|Montage|GetCurrentActiveMontage _returnvalue))
  (bind _returnvalue_4 (Math|Random|RandomInteger _returnvalue_2))
  (bind _output (Utilities|Array|Get(acopy) _jumpsections _returnvalue_4))
  (Utilities|IsValid _jumpsectionnotify
    (:Is%20Valid
      (if (Variables|Default|GetEnableComboPeriod)
        (|ParseIndexfromSectionName _output)
        (Class|AnimInstance|MontageSetNextSection _returnvalue (Animation|Montage|MontageGetCurrentSection _returnvalue _returnvalue_3) _output _returnvalue_3)))))

(fn CreateWeapon
  (params (Class :type Actor%20Class%20Reference))
  ;[0.15 0.15 0.15 0.5] 在0，0，0生成一把武器
  (bind _returnvalue (Game|SpawnActorfromClass Class (Math|Transform|MakeTransform "0, 0, 0") "Undefined" "MultiplyWithRoot" 0 0))
  (bind _asbp_weapon_actor (Utilities|Casting|CastToBP_WeaponActor _returnvalue))
  (Utilities|Array|Add (Variables|Default|GetEquippedWeapons) _asbp_weapon_actor))

(fn AttachWeapon
  (params (index :type Integer) (SocketName :type Name))
  ;[0.15 0.15 0.15 0.5] 设置当前武器，并且去除武器的所有附着关系
  (Utilities|IsValid (Variables|Default|GetCurrentWeapon)
    (:Is%20Valid
      (Transformation|DetachFromActor (Variables|Default|GetCurrentWeapon) "KeepRelative" "KeepWorld" "KeepWorld"))
    (:Is%20Not%20Valid
      _))
  (Variables|Default|SetCurrentWeapon (Utilities|Array|Get(acopy) (Variables|Default|GetEquippedWeapons) index))
  ;[0.15 0.15 0.15 0.5] 将武器吸附至玩家身上，Snap to target能够让武器吸附上去而非在脚下
  (Utilities|IsValid (Variables|Default|GetCurrentWeapon)
    (:Is%20Valid
      (Transformation|AttachComponentToComponent (Variables|Default|GetCurrentWeapon) (Variables|Character|GetMesh) SocketName "SnapToTarget" "SnapToTarget" "SnapToTarget" true)
      ;[0.15 0.15 0.15 0.5] 设置武器的上级为玩家
      (Actor|SetOwner (Variables|Default|GetCurrentWeapon) self))))

(fn PlayMaterialEffect
  (params (InLinearColor :type Linear%20Color%20Structure) (EffectDuration :type Float%20%28single-precision%29) (TargetMesh :type Mesh%20Component%20Object%20Reference))
  ;[0.15 0.15 0.15 0.5] 对应mesh的material的element 0
  (Rendering|Material|SetVectorParameterValueonMaterials TargetMesh "EffectColor" (Math|Conversions|ToVector(LinearColor) InLinearColor))
  (Rendering|Material|SetScalarParameterValueonMaterials TargetMesh "StartTime" (- (+ EffectDuration (Utilities|Time|GetTimeSeconds)) 1.0)))