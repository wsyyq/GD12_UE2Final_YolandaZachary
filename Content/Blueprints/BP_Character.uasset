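; Player character Blueprint with melee, roll, two cooldown skills (berserk, meteor damage box) and potion pickups, also driving start, HUD, mission menu and win screens.
; Health floors at 1 so Tick can trigger a one-shot death: respawn at the saved save-point transform, or reload the level.
; Kills and potions heal through HPUp, which updates the health bar.
; Movement speed and skill casts emit noise for enemy hearing.
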(event OnComponentBeginOverlap(Box)
  (params (OverlappedComponent :type Primitive%20Component%20Object%20Reference) (OtherActor :type Actor%20Object%20Reference) (OtherComp :type Primitive%20Component%20Object%20Reference) (OtherBodyIndex :type Integer) (bFromSweep :type Boolean) (SweepResult :type Hit%20Result%20Structure%20%28by%20ref%29))
  (Utilities|Casting|CastToBP_Goblin_BT OtherActor))

(event Custom|VFX_HPUp
  (bind _p_summon_parent_startup (Variables|Default|GetP_Summon_Parent_Startup))
  ;[0.149 0 0 0.502] 血量回复
  ;;[0.15 0.15 0.15 0.5] 拾取回血物品时播放特效
  (Development|SetHiddeninGame _p_summon_parent_startup false false)
  (Utilities|FlowControl|Delay 1.0)
  (Development|SetHiddeninGame _p_summon_parent_startup true false))

(event Custom|HPUp_AIDie
  ;[0.149 0 0 0.502] 血量回复
  ;;[0.15 0.15 0.15 0.5] 击杀敌人后回血30
  (CallFunction|HPUp 3e+01 (Variables|Default|GetHealth)))

(event Custom|Rebirth
  ;[0.15 0 0 0.5] 角色死亡与重生
  (Utilities|FlowControl|DoOnce false
    (:Completed
      (if (Variables|Default|GetCanRebirth)
        ;;[0.15 0.15 0.15 0.5] 角色死亡
        (Variables|Default|SetIsCharacterInvincible true)
        (Input|DisableInput (Game|GetPlayerController 0))
        (Animation|Montage|PlayMontage (Variables|Character|GetMesh) "/Game/Characters/Animations/AM_Death.AM_Death" 0.8
          (:then
            ;;[0.15 0.15 0.15 0.5] 时缓2s
            (Utilities|FlowControl|Delay 0.3)
            (Utilities|Time|SetGlobalTimeDilation 0.2)
            (Utilities|FlowControl|Delay 0.05)
            (Utilities|Time|SetGlobalTimeDilation 1.0)
            ;;[0.15 0.15 0.15 0.5] 重生
            (Transformation|SetActorTransform (Variables|Default|GetRebirthTransform) false true)
            (CallFunction|HPUp 1e+02 (Variables|Default|GetHealth))
            (Animation|Montage|PlayMontage (Variables|Character|GetMesh) "/Game/Characters/Animations/AM_Rebirth.AM_Rebirth"
              (:OnCompleted
                (Input|EnableInput (Game|GetPlayerController 0))
                (Variables|Default|SetIsCharacterInvincible false)))))
        (else
          ;;[0.15 0.15 0.15 0.5] 若无重生点，则重启
          (Variables|Default|SetIsCharacterInvincible true)
          (Input|DisableInput (Game|GetPlayerController 0))
          (Animation|Montage|PlayMontage (Variables|Character|GetMesh) "/Game/Characters/Animations/AM_Death.AM_Death"
            (:then
              (Audio|PlaySound2D "/Game/Assets/Sounds/UI/A_UI_GameOver01.A_UI_GameOver01" 1.0 1.0 0.0 0 0)
              (Utilities|FlowControl|Delay 3.0)
              (Utilities|Time|SetGlobalTimeDilation 0.1)
              (Utilities|FlowControl|Delay 0.2)
              (Utilities|Time|SetGlobalTimeDilation 1.0)
              (Game|OpenLevel(byName) "GD12_YolandaZachary_FinalMap"))))))))

(event Custom|StartLevel
  (bind _returnvalue (Game|GetPlayerController 0))
  ;[0.149 0 0 0.502] WBP
  ;;[0.149 0.149 0.149 0.502] 启动游戏时WBP
  (Widget|RemovefromParent (stale EventBeginPlay _returnvalue_3))
  (Variables|/Script/Engine.PlayerController|SetbShowMouseCursor _returnvalue false)
  (Input|SetInputModeGameOnly _returnvalue false)
  (bind _returnvalue_2 (Game|ConstructObjectfromClass "/Game/UI/WBP_InGame.WBP_InGame_C"))
  (UserInterface|Viewport|AddtoViewport _returnvalue_2 0)
  (Variables|Default|SetWBPInGame _returnvalue_2))

(event Custom|OpenWBPGameWin
  (bind _returnvalue (Game|GetPlayerController 0))
  ;[0.149 0 0 0.502] WBP
  ;;[0.149 0.149 0.149 0.502] 游戏胜利WBP
  (Utilities|FlowControl|Delay 3.5)
  (Widget|RemovefromParent (stale Custom|StartLevel _returnvalue_2))
  (bind _returnvalue_2 (Game|ConstructObjectfromClass "/Game/UI/WBP_GameWin.WBP_GameWin_C"))
  (UserInterface|Viewport|AddtoViewport _returnvalue_2 0)
  (Utilities|Time|SetGlobalTimeDilation 0.0)
  (Variables|/Script/Engine.PlayerController|SetbShowMouseCursor _returnvalue true)
  (Input|SetInputModeUIOnly _returnvalue _returnvalue_2 "DoNotLock" false)
  (EventDispatchers|BindEventtoEventGameStart _returnvalue_2 (delegate Custom|RestartLevel)))

(event Custom|RestartLevel
  ;[0.149 0 0 0.502] WBP
  ;;[0.149 0.149 0.149 0.502] 游戏胜利WBP
  (Widget|RemovefromParent (stale Custom|OpenWBPGameWin _returnvalue_2))
  (Variables|/Script/Engine.PlayerController|SetbShowMouseCursor (Game|GetPlayerController 0) false)
  (Input|SetInputModeGameOnly (Game|GetPlayerController 0) false)
  (Utilities|Time|SetGlobalTimeDilation 1.0)
  (Game|OpenLevel(byName) "GD12_YolandaZachary_FinalMap"))

(event Custom|Skill2InCD_ChangeWBP
  ;[0.15 0.007599 0 0.5] 玩家动作
  ;;[0.15 0.15 0.15 0.5] 技能2-对面前250*250*200的敌人造成100伤害，冷却30s，400噪音会吸引敌人
  (Variables|Skill1|SetIsSkill1CD true)
  (Default|SetSkill2State (Variables|Default|GetWBPInGame) false)
  (Utilities|FlowControl|Delay (Variables|Skill1|GetSkill1CD))
  (Variables|Skill1|SetIsSkill1CD false)
  (Default|SetSkill2State (Variables|Default|GetWBPInGame) true))

(event Custom|Skill1InCD_ChangeWBP
  ;[0.15 0.007599 0 0.5] 玩家动作
  ;;[0.15 0.15 0.15 0.5] 数字键1-狂暴, 持续7s，使用技能时身体会发紫光，冷却20s，400噪音会吸引敌人
  (Variables|Skill2|SetIsSkill2CD true)
  (Default|SetSkill1State (Variables|Default|GetWBPInGame) false)
  (Utilities|FlowControl|Delay (Variables|Skill2|GetSkill2CD))
  (Variables|Skill2|SetIsSkill2CD false)
  (Default|SetSkill1State (Variables|Default|GetWBPInGame) true))

(event EventBeginPlay
  (bind _returnvalue (Game|GetPlayerController 0))
  ;[0.15 0.15 0.15 0.5] 开始游戏不显示回血特效
  (|CallParentFunction)
  (Development|SetHiddeninGame (Variables|Default|GetP_Summon_Parent_Startup) true false)
  ;[0.15 0.15 0.15 0.5] 在收到攻击时血量不会归0（用于复活）
  (Variables|Default|SetMinHealth 1.0)
  (EventDispatchers|BindEventtoAIAlreadyDie (delegate Custom|HPUp_AIDie))
  (bind _returnvalue_2 (Actor|GetActorOfClass "/Game/Blueprints/Level/BP_Mission/BP_MissionManager.BP_MissionManager_C"))
  (EventDispatchers|BindEventtoMissionOver _returnvalue_2 (delegate Custom|OpenWBPGameWin))
  (Variables|Default|SetMissionManager _returnvalue_2)
  ;[0.149 0 0 0.502] WBP
  ;;[0.149 0.149 0.149 0.502] 启动游戏时WBP
  (bind _returnvalue_3 (Game|ConstructObjectfromClass "/Game/UI/WBP_GameStart.WBP_GameStart_C"))
  (UserInterface|Viewport|AddtoViewport _returnvalue_3 0)
  (Variables|/Script/Engine.PlayerController|SetbShowMouseCursor _returnvalue true)
  (Input|SetInputModeUIOnly _returnvalue _returnvalue_3 "DoNotLock" false)
  (EventDispatchers|BindEventtoEventGameStart _returnvalue_3 (delegate Custom|StartLevel))
  (Audio|PlaySound2D "/Game/Assets/Sounds/Ambient/A_Ambient_Wind02.A_Ambient_Wind02" 0.5 0.5 0.0 0 0))

(event Collision|EventActorBeginOverlap
  (params (OtherActor :type Actor%20Object%20Reference))
  (|CallParentFunction OtherActor) ; This node is disabled and will not be called.\nDrag off pins to build functionality.
)

(event EventOnDamaged
  (params (DamageAmount :type Float%20%28single-precision%29) (HitResult :type Hit%20Result%20Structure%20%28by%20ref%29) (InstigatorCharacter :type My%20ARPG%20Character%20Object%20Reference) (DamageCauser :type Actor%20Object%20Reference))
  ;[0.15 0.15 0.15 0.5] 受到伤害播放动画
  (|CallParentFunction DamageAmount HitResult InstigatorCharacter DamageCauser)
  (Utilities|Casting|CastToBP_Character InstigatorCharacter)
  (Animation|PlayAnimMontage "/Game/Characters/Animations/AM_React_Hit.AM_React_Hit" 1.0 "None"))

(event EventTick
  (params (DeltaSeconds :type Float%20%28single-precision%29))
  (|CallParentFunction DeltaSeconds)
  ;[0.15 0.15 0.15 0.5] 血量不足时复活
  (Math|Float|CompareFloat (Variables|Default|GetHealth) 1.1
    (:>
      ;[0.149 0.149 0.149 0.502] 根据速度来计算响度
      (Utilities|FlowControl|Delay 0.2 :!label _label)
      (Class|PawnNoiseEmitterComponent|MakeNoise (Variables|Default|GetPawnNoiseEmitter) self (Math|Vector|VectorLengthXY (Transformation|GetVelocity)) (Transformation|GetActorLocation)))
    (:==
      (goto _label))
    (:<
      (CallFunction|Rebirth))))

(event Game|Damage|EventAnyDamage
  (params (Damage :type Float%20%28single-precision%29) (DamageType :type Damage%20Type%20Object%20Reference) (InstigatedBy :type Controller%20Object%20Reference) (DamageCauser :type Actor%20Object%20Reference))
  ;[0.15 0.15 0.15 0.5] 受伤Debug
  (|CallParentFunction Damage DamageType InstigatedBy DamageCauser)
  (Development|PrintString (Utilities|String|Append "当前血量为" (Utilities|String|ToString(Float) (Variables|Default|GetHealth)))))

(event Input|ActionEvents|InputActionNormalAttack
  (params (Key :type Key%20Structure :default "None"))
  ;[0.15 0.007599 0 0.5] 玩家动作
  ;;[0.15 0.15 0.15 0.5] 鼠标左键-普通攻击
  (:Pressed
    (if (Variables|Skill1|GetIsInSkill1)
      (CallFunction|DoMeleeAttack 2.0)
      (else
        (CallFunction|DoMeleeAttack 1.3)))))

(event Input|ActionEvents|InputActionSprint
  (params (Key :type Key%20Structure :default "None"))
  (bind _charactermovement (Variables|Character|GetCharacterMovement))
  (bind _charactermovement_2 (Variables|Character|GetCharacterMovement))
  ;[0.15 0.007599 0 0.5] 玩家动作
  ;;[0.15 0.15 0.15 0.5] Shift-切换移动奔跑
  (:Pressed
    (if (Variables|Skill1|GetIsInSkill1)
      (Variables|/Script/Engine.CharacterMovementComponent|SetMaxWalkSpeed _charactermovement_2 8e+02)
      (else
        (Variables|/Script/Engine.CharacterMovementComponent|SetMaxWalkSpeed _charactermovement_2 6e+02))))
  (:Released
    (if (Variables|Skill1|GetIsInSkill1)
      (Variables|/Script/Engine.CharacterMovementComponent|SetMaxWalkSpeed _charactermovement 4e+02)
      (else
        (Variables|/Script/Engine.CharacterMovementComponent|SetMaxWalkSpeed _charactermovement 3e+02)))))

(event Input|ActionEvents|InputActionJump
  (params (Key :type Key%20Structure :default "None"))
  ;[0.15 0.007599 0 0.5] 玩家动作
  ;;[0.15 0.15 0.15 0.5] Space-跳跃，不能连跳
  (:Pressed
    (Utilities|FlowControl|DoOnce false :!label _label
      (:Completed
        (Character|Jump)
        (Utilities|FlowControl|Delay 0.5)
        (Character|StopJumping)
        (Utilities|FlowControl|Delay 1.0)
        (goto _label Reset)))))

(event Input|ActionEvents|InputActionSkillAttack1
  (params (Key :type Key%20Structure :default "None"))
  (bind _returnvalue (Game|GetPlayerController 0))
  (bind _skill1duration (Variables|Skill1|GetSkill1Duration))
  ;[0.15 0.007599 0 0.5] 玩家动作
  ;;[0.15 0.15 0.15 0.5] 数字键1-狂暴, 持续7s，使用技能时身体会发紫光，冷却20s，400噪音会吸引敌人
  (:Pressed
    (if (not (Variables|Skill2|GetIsSkill2CD))
      (CallFunction|Skill1inCDChangeWBP)
      (Animation|Montage|PlayMontage (Variables|Character|GetMesh) "/Game/Characters/Animations/AM_Skill_Combust.AM_Skill_Combust" 1.2
        (:then
          (Input|DisableInput _returnvalue)
          (Class|PawnNoiseEmitterComponent|MakeNoise (Variables|Default|GetPawnNoiseEmitter) self 4e+02 (Transformation|GetActorLocation)))
        (:OnCompleted
          (Input|EnableInput _returnvalue)
          (Development|PrintString "技能1进入狂暴")
          (Variables|Skill1|SetIsInSkill1 true)
          (CallFunction|PlayMaterialEffect "(R=0.143117,G=0.043877,B=1.000000,A=1.000000)" _skill1duration (Variables|Character|GetMesh))
          (Variables|Default|SetIsCharacterInvincible true)
          (Utilities|FlowControl|Delay _skill1duration)
          (Variables|Skill1|SetIsInSkill1 false)
          (Variables|Default|SetIsCharacterInvincible false)
          (Development|PrintString "狂暴结束"))
        (:OnInterrupted
          (Input|EnableInput _returnvalue))))))

(event Input|ActionEvents|InputActionRoll
  (params (Key :type Key%20Structure :default "None"))
  ;[0.15 0.007599 0 0.5] 玩家动作
  ;;[0.15 0.15 0.15 0.5] 鼠标右键-翻滚，不能连滚，滚时无敌
  (:Pressed
    (Utilities|FlowControl|DoOnce false :!label _label
      (:Completed
        (Variables|Default|SetCanRoll true)
        (Variables|Default|SetIsCharacterInvincible true)
        (Utilities|FlowControl|Delay 0.5)
        (Variables|Default|SetIsCharacterInvincible false)
        (Variables|Default|SetCanRoll false)
        (Utilities|FlowControl|Delay 1.0)
        (goto _label Reset)))))

(event Input|ActionEvents|InputActionPickUp
  (params (Key :type Key%20Structure :default "None"))
  (bind _returnvalue (Game|GetPlayerController 0))
  ;[0.15 0.007599 0 0.5] 玩家动作
  ;;[0.15 0.15 0.15 0.5] E-场景交互，播放动画（拾取物品与使用存档点）
  (:Pressed
    (for _array_element (Collision|GetOverlappingActors 0 :!class /Script/Engine.Actor)
      (if (Utilities|DoesObjectImplementInterface _array_element "/Game/Blueprints/Level/BI_Interact.BI_Interact_C")
        (bind _asbp_save_place (Utilities|Casting|CastToBP_SavePlace _array_element)
          (:then
            (Variables|Default|SetIsCharacterInvincible true)
            (bind _canpick (Class|BIInteract|E2Interact(Message) _asbp_save_place))
            (if _canpick
              (Input|DisableInput (Game|GetPlayerController 0))
              (Animation|Montage|PlayMontage (Variables|Character|GetMesh) "/Game/Characters/Animations/AM_Skill_Fireball.AM_Skill_Fireball"
                (:OnCompleted
                  (Input|EnableInput (Game|GetPlayerController 0))
                  (Variables|Default|SetIsCharacterInvincible false)
                  (Variables|Default|SetRebirthTransform (Transformation|GetActorTransform))
                  (Variables|Default|SetCanRebirth true)))))
          (:CastFailed
            (bind _asbp_potions (Utilities|Casting|CastToBP_Potions _array_element))
            (bind _canpick_2 (Class|BIInteract|E2Interact(Message) _asbp_potions))
            (if _canpick_2
              (Animation|Montage|PlayMontage (Variables|Character|GetMesh) "/Game/Characters/Animations/AM_Item_Potion_Mana.AM_Item_Potion_Mana"
                (:then
                  (Input|DisableInput _returnvalue))
                (:OnCompleted
                  (Input|EnableInput _returnvalue)
                  (CallFunction|HPUp 1e+02 (Variables|Default|GetHealth) :!label _label)
                  (Development|PrintString "角色使用血瓶回血"))
                (:OnInterrupted
                  (goto _label))))))))))

(event Input|ActionEvents|InputActionSkillAttack2
  (params (Key :type Key%20Structure :default "None"))
  (bind _returnvalue (Game|GetPlayerController 0))
  (bind _returnvalue_2 (Transformation|GetActorRotation))
  ;[0.15 0.007599 0 0.5] 玩家动作
  ;;[0.15 0.15 0.15 0.5] 技能2-对面前250*250*200的敌人造成100伤害，冷却30s，400噪音会吸引敌人
  (:Pressed
    (if (not (Variables|Skill1|GetIsSkill1CD))
      (CallFunction|Skill2inCDChangeWBP)
      (Animation|Montage|PlayMontage (Variables|Character|GetMesh) "/Game/Characters/Animations/AM_Skill_Meteor.AM_Skill_Meteor" 1.2
        (:then
          (Input|DisableInput _returnvalue)
          (Class|PawnNoiseEmitterComponent|MakeNoise (Variables|Default|GetPawnNoiseEmitter) self 4e+02 (Transformation|GetActorLocation))
          (bind _returnvalue_3 (Game|SpawnActorfromClass "/Game/Blueprints/Weapon/BP_Skill2Box.BP_Skill2Box_C" (Math|Transform|MakeTransform (+ (Transformation|GetActorLocation) (* (Math|Vector|GetForwardVector _returnvalue_2) 2e+02)) _returnvalue_2 "1.000000,1.000000,1.000000") "AlwaysSpawn" "MultiplyWithRoot" self 0))
          (Development|PrintString "释放陨石"))
        (:OnCompleted
          (Input|EnableInput _returnvalue :!label _label)
          (Actor|DestroyActor _returnvalue_3))
        (:OnInterrupted
          (goto _label))))))

(event Input|ActionEvents|InputActionOpenMenu
  (params (Key :type Key%20Structure :default "None"))
  ;[0.15 0.007599 0 0.5] 玩家动作
  ;;[0.15 0.15 0.15 0.5] Tab - Open Menu
  (:Pressed
    (if (Variables|Default|GetIsAlreadyOpenMenu)
      (Widget|RemovefromParent (stale _returnvalue))
      (Variables|Default|SetIsAlreadyOpenMenu false)
      (else
        (bind _returnvalue (Game|ConstructObjectfromClass "/Game/UI/WBP_TabMenu.WBP_TabMenu_C"))
        (UserInterface|Viewport|AddtoViewport _returnvalue 0)
        (Default|ResetMission _returnvalue (Utilities|Text|ToText(String) (.MissionDiscribe (Default|GetNowMission (Variables|Default|GetMissionManager)))))
        (Variables|Default|SetIsAlreadyOpenMenu true)
        (Audio|PlaySound2D "/Game/Assets/Sounds/UI/A_UI_WaveEnd.A_UI_WaveEnd" 0.8 0.8 0.0 0 0)))))

(fn ConstructionScript
  (|CallParentFunction))

(fn HPUp
  (params (AddHP :type Float%20%28double-precision%29) (OriHP :type Float%20%28double-precision%29))
  (bind _returnvalue (+ AddHP OriHP))
  (bind _maxhealth (Variables|Default|GetMaxHealth))
  (bind _playerwidget (Variables|Default|GetPlayerWidget))
  (bind _playerwidget_2 (Variables|Default|GetPlayerWidget))
  (CallFunction|VFXHPUp)
  (Math|Float|CompareFloat _returnvalue (Variables|Default|GetMaxHealth)
    (:>
      _)
    (:==
      _)
    (:<
      (bind _output_get (Variables|Default|SetHealth _returnvalue))
      (Development|PrintString (Utilities|String|Append "现在血量为" (Utilities|String|ToString(Float) _output_get)))
      ;[0.15 0.15 0.15 0.5] 更新血条值
      (Development|SetHiddeninGame _playerwidget_2 (not (CallFunction|IsAlive)) false)
      (bind _aswbp_player_ui (Utilities|Casting|CastToWBP_PlayerUI (UserInterface|GetWidget _playerwidget_2)))
      (Default|SetHPPercentage _aswbp_player_ui (/ (Variables|Default|GetHealth) (Variables|Default|GetMaxHealth)))
      (return _output_get)))
  (bind _output_get_2 (Variables|Default|SetHealth _maxhealth))
  (Development|PrintString (Utilities|String|Append "现在血量为" (Utilities|String|ToString(Float) _maxhealth)))
  ;[0.15 0.15 0.15 0.5] 更新血条值
  (Development|SetHiddeninGame _playerwidget (not (CallFunction|IsAlive)) false)
  (bind _aswbp_player_ui_2 (Utilities|Casting|CastToWBP_PlayerUI (UserInterface|GetWidget _playerwidget)))
  (Default|SetHPPercentage _aswbp_player_ui_2 (/ (Variables|Default|GetHealth) (Variables|Default|GetMaxHealth)))
  (return _output_get_2))